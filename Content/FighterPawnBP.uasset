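; FighterPawnBP is a fighter pawn that runs a scripted, timed demo of its action states once play begins.
; BeginPlay uses a chain of Delays to briefly pulse the hit, throwing and firing booleans in turn, then sets the dead flag permanently.
; The file does not read these flags, takes no input, and leaves Tick, overlap and the construction script empty.
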(event EventBeginPlay
  (Variables|Default|SetIsHit_0 true)
  (Utilities|FlowControl|Delay 0.1)
  (Variables|Default|SetIsHit_0 false)
  (Utilities|FlowControl|Delay 2.0)
  (Variables|Default|SetIsThrowing_0 true)
  (Utilities|FlowControl|Delay 0.1)
  (Variables|Default|SetIsThrowing_0 false)
  (Utilities|FlowControl|Delay 3.0)
  (Variables|Default|SetIsFiring_0 true)
  (Utilities|FlowControl|Delay 0.1)
  (Variables|Default|SetIsFiring_0 false)
  (Utilities|FlowControl|Delay 2.0)
  (Variables|Default|SetIsDead_0 true))

(event Collision|EventActorBeginOverlap
  (params (OtherActor :type Actor%20Object%20Reference)))

(event EventTick
  (params (DeltaSeconds :type Float%20%28single-precision%29)))

(fn ConstructionScript)